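; Openable door Blueprint that swings open and closed when its OpenDoor component sends open or close requests.
; On BeginPlay it caches its initial rotation and location.
; The DoorSwing timeline plays or reverses, adding a yaw curve to the starting rotation each update.
; A timeline event track plays the door lock sound at the cached location.
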(event OnOpenRequest(OpenDoor)
  (bind _door_rotation (Timeline|DoorSwing Play)
    (:Update
      (Transformation|SetActorRotation (Math|Rotator|CombineRotators (Math|Rotator|MakeRotator 0.0 0.0 _door_rotation) (Variables|Default|GetInitial%20Rotation))))
    (:Sound%20Timing
      (Audio|PlaySoundatLocation "/Game/Audio/door-lock.door-lock" (Variables|Default|GetDoor%20Location)))))

(event OnCloseRequest(OpenDoor)
  (bind _door_rotation (Timeline|DoorSwing Reverse)
    (:Update
      (Transformation|SetActorRotation (Math|Rotator|CombineRotators (Math|Rotator|MakeRotator 0.0 0.0 _door_rotation) (Variables|Default|GetInitial%20Rotation))))
    (:Sound%20Timing
      (Audio|PlaySoundatLocation "/Game/Audio/door-lock.door-lock" (Variables|Default|GetDoor%20Location)))))

(event EventBeginPlay
  (Variables|Default|SetInitial%20Rotation (Transformation|GetActorRotation))
  (Variables|Default|SetDoor%20Location (Transformation|GetActorLocation)))

(fn ConstructionScript)